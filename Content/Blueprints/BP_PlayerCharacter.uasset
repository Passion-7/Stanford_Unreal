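; Player character Blueprint that sets up the player's HUD and prints health values for debugging.
; On BeginPlay it creates a crosshair widget and a player health widget and adds both to the viewport.
; It prints the AttributeComp's Health every Tick and prints the new value whenever OnHealthChanged fires.
; The health widget receives no data from this graph, and the construction script is empty.
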(event `self.ReceiveBeginPlay`
  (bind _returnvalue (`|CreateWidget` "/Game/UI/Crosshair_Widget.Crosshair_Widget_C"))
  (`UserWidget.AddToViewport` _returnvalue 0)
  (bind _returnvalue_2 (`|CreateWidget` "/Game/UI/PlayerHealth_Widget.PlayerHealth_Widget_C"))
  (`UserWidget.AddToViewport` _returnvalue_2 0))

(event `self.ReceiveTick`
  (params (DeltaSeconds :type "Float (single-precision)"))
  (`KismetSystemLibrary.PrintString` (`KismetStringLibrary.Conv_DoubleToString` (`SAttributeComponent.Health` (`self.AttributeComp`))) true false (struct :`G` 0.66 :`B` 1.0 :`A` 1.0) 0.0))

(event `self.AttributeComp.OnHealthChanged`
  (params (InstigatorActor :type "Actor Object Reference") (OwningComp :type "SAttributeComponent Object Reference") (NewHealth :type "Float (single-precision)") (Delta :type "Float (single-precision)"))
  (`KismetSystemLibrary.PrintString` (`KismetStringLibrary.Conv_DoubleToString` NewHealth) true false (struct :`R` 1.0 :`G` 0.216577 :`A` 1.0)))

(fn `UserConstructionScript`)